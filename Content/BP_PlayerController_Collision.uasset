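; Player controller for inspecting collision by clicking on surfaces under the mouse cursor.
; On BeginPlay it shows the cursor, disables collision on the controlled pawn and adds the UI_CollisionShow widget to the viewport.
; Left click traces the Visibility channel under the cursor and draws a debug sphere at the impact point with an arrow along the surface normal.
; The F key toggles that trace between simple and complex collision.
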(event `self.ReceiveBeginPlay`
  (set `self.bShowMouseCursor` true)
  (`self.SetActorEnableCollision` (`self.K2_GetPawn`) false)
  (bind _returnvalue (`|CreateWidget` "/GeneratedComplexCollision/UI_CollisionShow.UI_CollisionShow_C" self))
  (`UserWidget.AddToViewport` _returnvalue 0))

(event `Key|LeftMouseButton`
  (params (Key :type "Key Structure"))
  (bind (_hitresult _returnvalue) (`self.GetHitResultUnderCursorByChannel` "TraceTypeQuery1" (`self.bTraceComplex`)))
  (bind (_bblockinghit _binitialoverlap _time _distance _location _impactpoint _normal _impactnormal) (`GameplayStatics.BreakHitResult` _hitresult))
  (:`Pressed`
    (if _returnvalue
      (`KismetSystemLibrary.DrawDebugSphere` _impactpoint 5.0 12 (struct :`R` 1.0 :`B` 0.038008 :`A` 1.0) 3.0)
      (`KismetSystemLibrary.DrawDebugArrow` _impactpoint (+ _impactpoint (* _impactnormal 30.0)) 10.0 (struct :`R` 0.042714 :`G` 1.0 :`A` 1.0) 3.0))))

(event `Key|F`
  (params (Key :type "Key Structure"))
  (:`Pressed`
    (set `self.bTraceComplex` (not (`self.bTraceComplex`)))))

(fn `UserConstructionScript`)